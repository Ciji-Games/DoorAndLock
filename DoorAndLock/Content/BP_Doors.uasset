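; BP_Doors is an interactive door the player toggles open and closed with E while inside its Box trigger, unless it is locked.
; Box overlaps enable and disable player input, and a FlipFlop plays or reverses a timeline driving SMDoor's absolute world yaw.
; The construction script colors a PointLight red when locked or green when unlocked.
; A disconnected chain of delayed debug prints never runs.
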(event `self.ReceiveBeginPlay`)

(event `self.ReceiveTick`
  (params (DeltaSeconds :type "Float (single-precision)")))

(event `self.Box.OnComponentBeginOverlap`
  (params (OverlappedComponent :type "PrimitiveComponent Object Reference") (OtherActor :type "Actor Object Reference") (OtherComp :type "PrimitiveComponent Object Reference") (OtherBodyIndex :type Integer) (bFromSweep :type Boolean) (SweepResult :type "HitResult Structure (by ref)"))
  (`self.EnableInput` (`GameplayStatics.GetPlayerController` 0)))

(event `self.Box.OnComponentEndOverlap`
  (params (OverlappedComponent :type "PrimitiveComponent Object Reference") (OtherActor :type "Actor Object Reference") (OtherComp :type "PrimitiveComponent Object Reference") (OtherBodyIndex :type Integer))
  (`self.DisableInput` (`GameplayStatics.GetPlayerController` 0)))

(event `Key|E`
  (params (Key :type "Key Structure"))
  (:`Pressed`
    (if (not (`self.IsLocked`))
      (`/Engine/EditorBlueprintResources/StandardMacros.FlipFlop`
        (:`A`
          (bind (_direction _rotation) (`Timeline|OpenCloseDoorTimeline` :!label _label)
            (:`Update`
              (`SceneComponent.K2_SetWorldRotation` (`self.SM_Door`) (`KismetMathLibrary.MakeRotator` 0.0 0.0 _rotation) false false))))
        (:`B`
          (goto _label :!via `Reverse`))))))

(fn `UpdateLight`
  (bind _pointlight (`self.PointLight`))
  (if (`self.IsLocked`)
    (`LightComponent.SetLightColor` _pointlight (struct :`R` 1.0 :`B` 0.010649 :`A` 1.0) true)
    (else
      (`LightComponent.SetLightColor` _pointlight (struct :`G` 1.0 :`B` 0.081891 :`A` 1.0) true))))

(fn `UserConstructionScript`
  (`self.UpdateLight`))