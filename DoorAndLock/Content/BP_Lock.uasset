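; BP_Lock is an interactable switch that inverts the lock state of a set of linked doors.
; Overlapping its Box enables input from player controller 0, and leaving disables it.
; Pressing E increments a counter shown on a TextRender, then flips IsLocked on each entry in the Doors array and calls UpdateLight on it.
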(event `self.Box.OnComponentBeginOverlap`
  (params (OverlappedComponent :type "PrimitiveComponent Object Reference") (OtherActor :type "Actor Object Reference") (OtherComp :type "PrimitiveComponent Object Reference") (OtherBodyIndex :type Integer) (bFromSweep :type Boolean) (SweepResult :type "HitResult Structure (by ref)"))
  (`self.EnableInput` (`GameplayStatics.GetPlayerController` 0)))

(event `self.Box.OnComponentEndOverlap`
  (params (OverlappedComponent :type "PrimitiveComponent Object Reference") (OtherActor :type "Actor Object Reference") (OtherComp :type "PrimitiveComponent Object Reference") (OtherBodyIndex :type Integer))
  (`self.DisableInput` (`GameplayStatics.GetPlayerController` 0)))

(event `Key|E`
  (params (Key :type "Key Structure"))
  ;[0.1285 0.15 0 0.5] Invert all lock status
  (:`Pressed`
    (bind _result (`/Engine/EditorBlueprintResources/StandardMacros.IncrementInt` (`self.Counter`))
      (:`  `
        (`TextRenderComponent.K2_SetText` (`self.TextRender`) (`KismetTextLibrary.Conv_IntToText` _result))
        (for _array_element (`self.Doors`)
          (set `/Game/BP_Doors.IsLocked` (not (`/Game/BP_Doors.IsLocked` _array_element)) _array_element)
          (`/Game/BP_Doors.UpdateLight` _array_element))))))

(fn `UserConstructionScript`)